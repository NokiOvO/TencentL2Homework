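; BP_MonsterTarget is a monster target that awards score when damaged through a player controller.
; AnyDamage casts the instigator to MyPlayerController, increments the score on its MyPlayerState, then plays a damage animation and returns to the looping run after a short delay.
; A test input also plays the damage animation.
; Timeline logic for moving the skeletal mesh along a spline exists but is unconnected and never runs.
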(event `InputAction|test`
  (params (Key :type "Key Structure"))
  (:`Pressed`
    (`SkeletalMeshComponent.PlayAnimation` (`self.SkeletalMesh`) "/Game/Yippy_Kawaii/Animations/Anim_Damage.Anim_Damage" false)))

(event `self.ReceiveAnyDamage`
  (params (Damage :type "Float (single-precision)") (DamageType :type "DamageType Object Reference") (InstigatedBy :type "Controller Object Reference") (DamageCauser :type "Actor Object Reference"))
  (bind _asmy_player_controller (cast `/Game/Blueprints/MyPlayerController` InstigatedBy))
  (bind _asmy_player_state (cast `/Game/Blueprints/MyPlayerState` (`Controller.PlayerState` _asmy_player_controller)))
  (`/Game/Blueprints/MyPlayerState.IncrementScore` _asmy_player_state)
  (`self.PlayAnim`))

(event `PlayAnim`
  (`SkeletalMeshComponent.PlayAnimation` (`self.SkeletalMesh`) "/Game/Yippy_Kawaii/Animations/Anim_Damage.Anim_Damage" false)
  (`KismetSystemLibrary.Delay` 0.6)
  (`SkeletalMeshComponent.PlayAnimation` (`self.SkeletalMesh`) "/Game/Yippy_Kawaii/Animations/Anim_Run.Anim_Run" true))

(fn `UserConstructionScript`)