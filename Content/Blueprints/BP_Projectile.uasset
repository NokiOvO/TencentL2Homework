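; Projectile that plays a pitch-randomized impact sound on hit, damages monster targets and knocks hats off characters.
; A component tagged "Hat" on a Character switches to physics, takes a fraction of the projectile's velocity plus random spin, and plays a second, quieter sound.
; Other hits spawn a particle effect, with damage applied only to non-Character BP_MonsterTarget actors; the random character-damage branch is disconnected.
; The projectile destroys itself on every hit.
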(event `self.ReceiveHit`
  (params (MyComp :type "PrimitiveComponent Object Reference") (Other :type "Actor Object Reference") (OtherComp :type "PrimitiveComponent Object Reference") (bSelfMoved :type Boolean) (HitLocation :type "Vector Structure") (HitNormal :type "Vector Structure") (NormalImpulse :type "Vector Structure") (Hit :type "HitResult Structure (by ref)"))
  ;[0 1 0] Sound
  (`GameplayStatics.PlaySoundAtLocation` "/Game/Sounds/SoundCue_Attentuated.SoundCue_Attentuated" HitLocation (struct) (`self.VolumeMultiplier`) (`KismetMathLibrary.RandomFloatInRange` 0.8 1.2) 0.0 null null null)
  (cast `Character` Other
    (:`then`
      (if (`ActorComponent.ComponentHasTag` OtherComp "Hat")
        ;[1 1 1] Hit Hat
        (`self.K2_DestroyActor`)
        (`PrimitiveComponent.SetSimulatePhysics` OtherComp true)
        (`PrimitiveComponent.SetPhysicsLinearVelocity` OtherComp (/ (`MovementComponent.Velocity` (`self.ProjectileMovement`)) 3.0) false "None")
        (`PrimitiveComponent.SetPhysicsAngularVelocityInDegrees` OtherComp (`KismetMathLibrary.MakeVector` (`KismetMathLibrary.RandomFloatInRange` -720.0 720.0) (`KismetMathLibrary.RandomFloatInRange` -720.0 720.0) (`KismetMathLibrary.RandomFloatInRange` -720.0 720.0)) false "None")
        ;[0 1 0] Sound
        (`GameplayStatics.PlaySoundAtLocation` "/Game/Sounds/Randomize_01.Randomize_01" HitLocation (struct) (* (`self.VolumeMultiplier`) 0.25) 1.0 0.0 null null null)
        (else
          (`self.K2_DestroyActor` :!label _label)
          (`GameplayStatics.SpawnEmitterAtLocation` "/Game/Effects/P_Hit.P_Hit" HitLocation))))
    (:`CastFailed`
      ;[1 1 1] Hit Character
      (bind _asbp_monster_target (cast `/Game/Blueprints/BP_MonsterTarget` Other)
        (:`then`
          (`GameplayStatics.ApplyDamage` _asbp_monster_target 1.0 (`self.GetInstigatorController`) self)
          (goto _label))
        (:`CastFailed`
          (goto _label))))))

(fn `UserConstructionScript`)